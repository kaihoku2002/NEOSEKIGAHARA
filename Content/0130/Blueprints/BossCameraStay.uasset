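; Boss encounter trigger that plays the BossStartMovie intro when the player first overlaps it, then becomes the fight's view target.
; On overlap it switches on BP_SplineCamera's air wall, disables player input and plays the sequence with BP_OdaNobunaga bound by the "Boss" tag.
; When the sequence finishes it restores input, blends the view to itself through BP_TGS_GameMode, creates the boss widget and switches the air wall off.
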(event Custom|CustomEvent
  (Input|EnableInput (Game|GetPlayerCharacter 0) 0)
  (bind _asbp_tgs_game_mode (Utilities|Casting|CastToBP_TGS_GameMode (Game|GetGameMode)))
  (Class|TGSGameMode|SetViewTargetwithBlend _asbp_tgs_game_mode self 0.0 "VTBlend_Linear" 0.0 false)
  (bind _returnvalue (Actor|GetActorOfClass "/Game/0113/BOSS/BP_OdaNobunaga.BP_OdaNobunaga_C"))
  (Default|WidgetCreate _returnvalue)
  (bind _returnvalue_2 (Actor|GetActorOfClass "/Game/0130/Blueprints/BP_SplineCamera.BP_SplineCamera_C"))
  (Default|AirWallSwitch _returnvalue_2 false))

(event EventBeginPlay
  (|CallParentFunction) ; このノードは無効になっているため呼び出せません。\n機能をビルドするにはピンをドラッグしてください。
)

(event Collision|EventActorBeginOverlap
  (params (OtherActor :type Actor%20Object%20Reference))
  (if (Actor|ActorHasTag OtherActor "Player")
    (Utilities|FlowControl|DoOnce false
      (:Completed
        (bind _returnvalue (Actor|GetActorOfClass "/Game/0130/Blueprints/BP_SplineCamera.BP_SplineCamera_C"))
        (Default|AirWallSwitch _returnvalue true)
        (Input|DisableInput (Game|GetPlayerCharacter 0) 0)
        (bind (_outactor _returnvalue_2) (Sequencer|Player|CreateLevelSequencePlayer "/Game/0122/Level/BossStartMovie.BossStartMovie" (Utilities|Struct|MakeMovieSceneSequencePlaybackSettings false "(Value=0)")))
        (EventDispatchers|BindEventtoOnFinished _returnvalue_2 (delegate Custom|CustomEvent))
        (Utilities|FlowControl|Sequence
          (:then_0
            (bind _returnvalue_3 (Actor|GetActorOfClass "/Game/0113/BOSS/BP_OdaNobunaga.BP_OdaNobunaga_C"))
            (Class|LevelSequenceActor|AddBindingbyTag _outactor "Boss" _returnvalue_3 false))
          (:then_1
            (Sequencer|Player|Play _returnvalue_2 :!class /Script/MovieScene.MovieSceneSequencePlayer)))))))

(event EventTick
  (params (DeltaSeconds :type Float%20%28single-precision%29))
  (|CallParentFunction DeltaSeconds) ; このノードは無効になっているため呼び出せません。\n機能をビルドするにはピンをドラッグしてください。
)

(fn ConstructionScript
  (|CallParentFunction))
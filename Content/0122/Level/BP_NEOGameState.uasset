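; Game state Blueprint that drives the title, demo, opening and game-over screens.
; BeginPlay creates the widgets and looping-ambience sound components, then sets the view to the title camera.
; Tick polls the game and title states, using DoOnce gates to show each screen, except the demo widget, which is re-added directly.
; A timer switches title to demo and resets its gate; DeleteWidget clears the title screen, timer and ambience.
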(event EventBeginPlay
  (bind _returnvalue (UserInterface|CreateWidget "/Game/0122/Level/nitidenMovie/BP_NitidenLogo.BP_NitidenLogo_C"))
  (Variables|Default|SetLogoWidget _returnvalue)
  (bind _returnvalue_2 (UserInterface|CreateWidget "/Game/0122/BP_TitleLogo.BP_TitleLogo_C"))
  (Variables|Default|SetTitleWidget _returnvalue_2)
  (bind _returnvalue_3 (UserInterface|CreateWidget "/Game/0122/Level/DemoMovie/BP_Demo.BP_Demo_C"))
  (Variables|Default|SetDemoWidget _returnvalue_3)
  (bind _returnvalue_4 (UserInterface|CreateWidget "/Game/0130/Level/Weight_GameOver.Weight_GameOver_C"))
  (Variables|Default|SetOverWidget _returnvalue_4)
  (bind _returnvalue_5 (Actor|GetActorOfClass "/Game/0130/Blueprints/BP_SplineCamera.BP_SplineCamera_C"))
  (Class|SplineCamera|SetPlayerCamera _returnvalue_5)
  (bind _returnvalue_6 (Actor|GetActorOfClass "/Game/0122/Level/TitleCamera.TitleCamera_C"))
  (Game|Player|SetViewTargetwithBlend (Game|GetPlayerController 0) _returnvalue_6 0.0 "VTBlend_Linear" 0.0 false)
  (bind _returnvalue_7 (Audio|CreateSound2D "/Game/0102/SE/Flagbatbata.Flagbatbata" 1.0 1.0 0.0 0))
  (Variables|Default|SetFlag _returnvalue_7)
  (bind _returnvalue_8 (Audio|CreateSound2D "/Game/0102/SE/LongAir.LongAir" 1.0 1.0 0.0 0))
  (Variables|Default|SetWind _returnvalue_8))

(event EventTick
  (params (DeltaSeconds :type Float%20%28single-precision%29))
  (switch Utilities|FlowControl|Switch|SwitchonEGameState_NEO (Class|NEOGameState|GetGameState)
    (:OnTitle
      (CallFunction|OnGameTitle))
    (:OnOpening
      (Utilities|FlowControl|DoOnce false
        (:Completed
          (bind _returnvalue (UserInterface|CreateWidget "/Game/0130/Level/Widget_GameOpening.Widget_GameOpening_C"))
          (UserInterface|Viewport|AddtoViewport _returnvalue 0))))
    (:OnGameOver
      (Utilities|FlowControl|DoOnce false
        (:Completed
          (bind _returnvalue_2 (UserInterface|CreateWidget "/Game/0102/Movies/MediaGameOver.MediaGameOver_C"))
          (UserInterface|Viewport|AddtoViewport _returnvalue_2 0)
          (Utilities|FlowControl|Delay 2.0)
          (Audio|PlaySound2D "/Game/0102/SE/munen.munen" 1.0 1.0 0.0 0 0))))))

(event EventDeleteWidget
  (bind _wind (Variables|Default|GetWind))
  (bind _flag (Variables|Default|GetFlag))
  (Utilities|Time|ClearandInvalidateTimerbyHandle (stale EventDisplayTitleScreen _returnvalue))
  (if (Audio|Components|Audio|IsPlaying _flag)
    (Audio|Components|Audio|Stop _flag))
  (if (Audio|Components|Audio|IsPlaying _wind)
    (Audio|Components|Audio|Stop _wind))
  (Widget|RemovefromParent (Variables|Default|GetTitleWidget)))

(event EventDisplayDemoScreen
  (Utilities|Time|ClearandInvalidateTimerbyHandle (stale EventDisplayTitleScreen _returnvalue))
  (Widget|RemovefromParent (Variables|Default|GetTitleWidget))
  (Class|NEOGameState|SetTitleState "OnDemoDisplay")
  (Utilities|FlowControl|DoOnce false) ; enters at Reset
)

(event EventDisplayTitleScreen
  (Utilities|FlowControl|DoOnce false
    (:Completed
      (UserInterface|Viewport|AddtoViewport (Variables|Default|GetTitleWidget) 0)
      (Audio|PlaySound2D "/Game/0102/SE/NEO_SEKIGAHARA.NEO_SEKIGAHARA" 1.0 1.0 0.0 0 0)
      (Audio|Components|Audio|Play (Variables|Default|GetWind) 0.0)
      (Audio|Components|Audio|Play (Variables|Default|GetFlag) 0.0)
      (bind _returnvalue (Utilities|Time|SetTimerbyEvent (delegate EventDisplayDemoScreen) 15.0)))))

(fn ConstructionScript)

(fn OnGameTitle
  (switch Utilities|FlowControl|Switch|SwitchonETitleState_NEO (Class|NEOGameState|GetTitleState)
    (:OnTitleDisplay
      (Class|NEOGameState|DisplayTitleScreen))
    (:OnDemoDisplay
      (UserInterface|Viewport|AddtoViewport (Variables|Default|GetDemoWidget) 0))))
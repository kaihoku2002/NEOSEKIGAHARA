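; BP_NEOGameMode is a game mode that drives a screen fade transition based on whether the game is in a battle area.
; BeginPlay creates a BP_Black widget, stored as Smoke.
; Tick polls GetIsBattleArea, using paired DoOnce gates to add and fade in the widget when true, then fade it out and remove it once false.
; Each finished animation resets the other gate, and DestroyerEvent is empty.
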(event EventBeginPlay
  (bind _returnvalue (UserInterface|CreateWidget "/Game/0122/Level/BP_Black.BP_Black_C"))
  (Variables|Default|SetSmoke _returnvalue))

(event EventTick
  (params (DeltaSeconds :type Float%20%28single-precision%29))
  (bind _smoke (Variables|Default|GetSmoke))
  (if (Class|NEOGameMode|GetIsBattleArea)
    (Utilities|FlowControl|DoOnce false :!label _label
      (:Completed
        (UserInterface|Viewport|AddtoViewport _smoke 0)
        (Components|Animation|PlayAnimation _smoke (Variables|/Game/0122/Level/BP_Black.BP_Black_C|GetFadein _smoke) 0.0
          (:Finished
            (goto _label_2 Reset)))))
    (else
      (Utilities|FlowControl|DoOnce true :!label _label_2
        (:Completed
          (Components|Animation|PlayAnimation _smoke (Variables|/Game/0122/Level/BP_Black.BP_Black_C|GetFadeOut _smoke) 0.0
            (:Finished
              (Widget|RemovefromParent _smoke)
              (goto _label Reset))))))))

(event EventDestroyerEvent)

(fn ConstructionScript)